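; Base interactable item actor for the RPG item system that shows item info on proximity and can be picked up.
; The construction script fills ItemInfo from the ItemDT data table, using the ItemName enum as the row name.
; Sphere overlaps toggle the item message on the overlapping actor, with display gated by Interactable.
; When Interactable, Interact sends ItemInfo to player 0's PickupMessage and destroys the actor if Destroy is set.
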(event `/Game/RPG/ItemSys/Blueprints/ChInterface_BPI.Interact`
  (if (`self.Interactable?`)
    (message `/Game/RPG/ItemSys/Blueprints/ChInterface_BPI.Pickup` (`GameplayStatics.GetPlayerCharacter` 0) (`self.ItemInfo`))
    (if (`self.Destroy?`)
      (`self.K2_DestroyActor`))))

(event `self.Sphere.OnComponentBeginOverlap`
  (params (OverlappedComponent :type "PrimitiveComponent Object Reference") (OtherActor :type "Actor Object Reference") (OtherComp :type "PrimitiveComponent Object Reference") (OtherBodyIndex :type Integer) (bFromSweep :type Boolean) (SweepResult :type "HitResult Structure (by ref)"))
  (if (`self.Interactable?`)
    (message `/Game/RPG/ItemSys/Blueprints/ChInterface_BPI.DisplayItem` OtherActor (`self.ItemInfo`) true)))

(event `self.Sphere.OnComponentEndOverlap`
  (params (OverlappedComponent :type "PrimitiveComponent Object Reference") (OtherActor :type "Actor Object Reference") (OtherComp :type "PrimitiveComponent Object Reference") (OtherBodyIndex :type Integer))
  (message `/Game/RPG/ItemSys/Blueprints/ChInterface_BPI.DisplayItem` OtherActor (`self.ItemInfo`) false))

(fn `UserConstructionScript`
  (bind _returnvalue (`|GetDataTableRow` "/Game/RPG/ItemSys/ItemDT.ItemDT" (`KismetStringLibrary.Conv_StringToName` (`|GetEnumeratorNameAsString` (`self.ItemName`))))
    (:`then`
      (set `self.ItemInfo` _returnvalue))))